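; Golf ball pawn that yaws its spring arm every tick from a turn value.
; Tick also passes the forward force to a debug text print, with both screen and log output switched off.
; A visibility collider is intended to handle the ball going behind walls, but its overlap events are unimplemented stubs marked with a TODO.
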(event OnComponentBeginOverlap(VisibilityCheckCollider)
  (params (OverlappedComponent :type Primitive%20Component%20Object%20Reference) (OtherActor :type Actor%20Object%20Reference) (OtherComp :type Primitive%20Component%20Object%20Reference) (OtherBodyIndex :type Integer) (bFromSweep :type Boolean) (SweepResult :type Hit%20Result%20Structure%20%28by%20ref%29))
  ;[1 1 1] TODO: Set visibility when ball is behind wall
)

(event OnComponentEndOverlap(VisibilityCheckCollider)
  (params (OverlappedComponent :type Primitive%20Component%20Object%20Reference) (OtherActor :type Actor%20Object%20Reference) (OtherComp :type Primitive%20Component%20Object%20Reference) (OtherBodyIndex :type Integer))
  ;[1 1 1] TODO: Set visibility when ball is behind wall
)

(event EventBeginPlay)

(event Collision|EventActorBeginOverlap
  (params (OtherActor :type Actor%20Object%20Reference)))

(event EventTick
  (params (DeltaSeconds :type Float%20%28single-precision%29))
  (CallFunction|DebugForce)
  (CallFunction|RotatePawn))

(fn ConstructionScript)

(fn RotatePawn
  (Transformation|AddLocalRotation (Variables|Default|GetSpringArm) (Math|Rotator|MakeRotator 0.0 0.0 (* (Input|AxisValues|GetTurn) 2.0)) false false))

(fn DebugForce
  (Development|PrintText (Utilities|Text|ToText(Float) (Class|BasePawn|GetForwardForce) "HalfToEven") false false))